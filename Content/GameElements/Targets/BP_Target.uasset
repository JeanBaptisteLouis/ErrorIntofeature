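; Shootable target, colored as good or bad, that scales in, flashes when hit, then scales out and spawns a replacement with the same settings.
; Moves by rotating the actor, with optional Perlin-noise wander and interpolated look-at to follow or avoid the player's aim point on a sphere.
; Aim comes from a reversed camera trace.
; An avoidance helper also repels it from its nearest neighbor and, in Avoid mode, a fixed point below.
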(event EventBeginPlay
  (bind _staticmesh (Variables|Default|GetStaticMesh))
  (Utilities|FlowControl|Sequence
    (:then_0
      (bind _returnvalue (Rendering|Material|CreateDynamicMaterialInstance (Rendering|Material|GetOverlayMaterial _staticmesh :!class /Script/Engine.MeshComponent) "None" "None" :!class /Script/Engine.KismetMaterialLibrary))
      (bind _output_get (Variables|Default|SetMat _returnvalue))
      (Rendering|Material|SetOverlayMaterial _staticmesh _output_get :!class /Script/Engine.MeshComponent)
      (Variables|Default|SetRelative%20Rotation (Variables|/Script/Engine.SceneComponent|GetRelativeRotation (Variables|Default|GetSpringArm))))
    (:then_1
      (bind (_direction _alpha) (Timeline|TM_Apparition PlayFromStart)
        (:Update
          (Transformation|SetRelativeScale3D (Variables|Default|GetScene) (Math|Conversions|ToVector(Float) _alpha)))
        (:Finished
          (switch Utilities|FlowControl|Switch|SwitchonETimelineDirection _direction
            (:Backward
              (Game|SpawnActorfromClass "BP_Target_C" (Math|Transform|MakeTransform "0, 0, 0" "0, 0, 0" "1.000000,1.000000,1.000000") "AlwaysSpawn" "MultiplyWithRoot" 0 (Variables|Default|GetBadTarget) (Variables|Default|GetMode) (Variables|Default|GetRandomMove) (Variables|Default|GetisBig) 0)
              (Actor|DestroyActor))))))))

(event EventTick
  (params (DeltaSeconds :type Float%20%28single-precision%29))
  (bind _returnvalue (Transformation|GetActorTransform))
  (Variables|Default|SetTargetLoc (Transformation|GetWorldLocation (Variables|Default|GetStaticMesh)))
  (bind _output_get (Variables|Default|SetHitIntensity (Math|Interpolation|FInterpTo (Variables|Default|GetHitIntensity) 0.0 DeltaSeconds 1e+01)))
  (Rendering|Material|SetScalarParameterValue (Variables|Default|GetMat) "Intensity" _output_get :!class /Script/Engine.MaterialInstanceDynamic)
  (Utilities|FlowControl|Sequence
    (:then_0
      (if (Variables|Default|GetRandomMove)
        (CallFunction|RandomMovement 2e+01)))
    (:then_1
      (bind _location (CallFunction|GetMousePointonSphere))
      (bind _output_get_2 (Variables|Default|SetAimLocation _location))
      (switch Utilities|FlowControl|Switch|SwitchonENUM_TargetMode (Variables|Default|GetMode)
        (:NewEnumerator0
          (Transformation|SetActorTransform (Class|KismetMathLibrary|TInterpto _returnvalue (Class|KismetAnimationLibrary|Lookat _returnvalue (Variables|Default|GetAimLocation) "-1.000000,0.000000,0.000000" false "0.000000,0.000000,1.000000" 0.0) (Utilities|Time|GetWorldDeltaSeconds) 1.0)))
        (:NewEnumerator1
          (CallFunction|Avoid _output_get_2 5e+02 1.0)
          (CallFunction|Avoid "0.000000,0.000000,-1500.000000" 2e+03 5.0))))
    (:then_2
      (bind _outactors (Actor|GetAllActorsOfClass "BP_Target_C"))
      (bind _nearesttarget (CallFunction|NearestTarget _outactors))
      (Utilities|IsValid _nearesttarget
        (:Is%20Valid
          (CallFunction|Avoid (Variables|BP_Target_C|GetTargetLoc _nearesttarget) 6e+02 (Math|Float|SelectFloat 3.0 1.0 (Variables|BP_Target_C|GetisBig _nearesttarget))))))))

(event EventBulletHit
  (Variables|Default|SetHitIntensity 3.0)
  (Collision|SetActorEnableCollision false)
  (Utilities|FlowControl|Sequence
    (:then_0
      (bind (_direction _alpha) (Timeline|TM_Apparition ReverseFromEnd)
        (:Update
          (Transformation|SetRelativeScale3D (Variables|Default|GetScene) (Math|Conversions|ToVector(Float) _alpha)))
        (:Finished
          (switch Utilities|FlowControl|Switch|SwitchonETimelineDirection _direction
            (:Backward
              (Game|SpawnActorfromClass "BP_Target_C" (Math|Transform|MakeTransform "0, 0, 0" "0, 0, 0" "1.000000,1.000000,1.000000") "AlwaysSpawn" "MultiplyWithRoot" 0 (Variables|Default|GetBadTarget) (Variables|Default|GetMode) (Variables|Default|GetRandomMove) (Variables|Default|GetisBig) 0)
              (Actor|DestroyActor))))))))

(fn ConstructionScript
  (Transformation|SetRelativeScale3D (Variables|Default|GetStaticMesh) (Math|Vector|SelectVector "3.000000,3.000000,3.000000" "1.000000,1.000000,1.000000" (Variables|Default|GetisBig)))
  (Transformation|SetActorRotation (Math|Rotator|MakeRotator 0.0 (Math|Random|RandomFloatinRange -45.0 -1e+01) (Math|Random|RandomFloatinRange 0.0 3.6e+02)))
  (Variables|Default|SetCoolRandomOffset (Math|Random|RandomFloatinRange 0.0 1e+03))
  (Rendering|Material|SetVectorParameterValueonMaterials (Variables|Default|GetStaticMesh) "Color" (Math|Conversions|ToVector(LinearColor) (Math|Color|SelectColor "(R=1.000000,G=0.000000,B=0.000000,A=1.000000)" "(R=0.034847,G=1.000000,B=0.078516,A=1.000000)" (Variables|Default|GetBadTarget)))))

(fn Avoid
  (params (LocationToAvoid :type Vector) (Radius :type Float%20%28double-precision%29) (Strength :type Float%20%28double-precision%29))
  (bind _returnvalue (Transformation|GetActorTransform))
  (bind _returnvalue_2 (Math|Float|MakeLiteralFloat Radius))
  (bind _staticmesh (Variables|Default|GetStaticMesh))
  (bind _returnvalue_3 (Transformation|GetWorldLocation _staticmesh))
  (if (<= (Math|Vector|Distance(Vector) LocationToAvoid _returnvalue_3) _returnvalue_2)
    (Transformation|SetActorTransform (Class|KismetMathLibrary|TInterpto _returnvalue (Class|KismetAnimationLibrary|Lookat _returnvalue (+ LocationToAvoid (* (Math|Vector|Normalize (- _returnvalue_3 LocationToAvoid)) _returnvalue_2)) "-1.000000,0.000000,0.000000" false "0.000000,0.000000,1.000000" 0.0) (Utilities|Time|GetWorldDeltaSeconds) (Math|Float|MakeLiteralFloat Strength)))))

(fn NearestTarget
  (params (Array :type Array%20of%20BP%20Target%20Object%20References))
  (bind _output_get (LocalVariables|SetTargets Array))
  (Utilities|Array|RemoveItem _output_get self)
  (LocalVariables|SetClosest (.OutItem (Utilities|Array|Random (LocalVariables|GetTargets))))
  (for _array_element (LocalVariables|GetTargets)
    (if (< (Math|Vector|Distance(Vector) (Variables|BP_Target_C|GetTargetLoc _array_element) (Variables|Default|GetTargetLoc)) (Math|Vector|Distance(Vector) (Variables|BP_Target_C|GetTargetLoc (LocalVariables|GetClosest)) (Variables|Default|GetTargetLoc)))
      (LocalVariables|SetClosest _array_element)))
  (return (LocalVariables|GetClosest)))

(fn GetMousePointonSphere
  (bind _asbp_player (Utilities|Casting|CastToBP_Player (Game|Player|GetPlayerPawn 0))
    (:then
      (bind _outhit (Collision|LineTraceByChannel (+ (* (Math|Vector|GetForwardVector (Variables|/Game/Player/BP_Player.BP_Player_C|GetCamera _asbp_player)) 1e+04) (Transformation|GetWorldLocation (Variables|/Game/Player/BP_Player.BP_Player_C|GetCamera _asbp_player))) (Transformation|GetWorldLocation (Variables|/Game/Player/BP_Player.BP_Player_C|GetCamera _asbp_player)) "TraceTypeQuery3" false 0 "None")))
    (:CastFailed
      _))
  (return (.Location (Collision|BreakHitResult _outhit))))

(fn RandomMovement
  (params (Strength :type Float%20%28double-precision%29))
  (bind _returnvalue (Utilities|Time|GetWorldDeltaSeconds))
  (bind _returnvalue_2 (Utilities|Time|GetTimeSeconds))
  (bind _coolrandomoffset (Variables|Default|GetCoolRandomOffset))
  (bind _returnvalue_3 (* _returnvalue_2 0.5))
  (Class|Actor|AddActorWorldRotation (Math|Rotator|MakeRotator 0.0 (* _returnvalue (Class|KismetMathLibrary|PerlinNoise1D (+ _returnvalue_3 (/ _coolrandomoffset 2.0))) Strength) (* _returnvalue (Class|KismetMathLibrary|PerlinNoise1D (+ _returnvalue_3 _coolrandomoffset)) Strength))))