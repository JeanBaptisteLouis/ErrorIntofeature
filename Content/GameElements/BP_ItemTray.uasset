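; Item tray for a flower task, with a child-actor button that validates the actors inside its detection volume.
; A press pushes a TaskManager tag for each wrong case, while a lone flower of the target (blue) color calls LevelFailed.
; Overlaps update the contents, toggle the button under optional count rules and trigger one-shot voice lines.
; When an incorrect-task response completes, it destroys everything inside except the player.
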(event OnComponentBeginOverlap(ItemDetection)
  (params (OverlappedComponent :type Primitive%20Component%20Object%20Reference) (OtherActor :type Actor%20Object%20Reference) (OtherComp :type Primitive%20Component%20Object%20Reference) (OtherBodyIndex :type Integer) (bFromSweep :type Boolean) (SweepResult :type Hit%20Result%20Structure%20%28by%20ref%29))
  (Utilities|Array|Add (Variables|Default|GetInTrayActors) OtherActor)
  (CallFunction|ManageActivatedonItemEnter)
  (CallFunction|PlaySoundifOnlyBlueFlower)
  (CallFunction|PlaySoundifAllFlowersin))

(event OnComponentEndOverlap(ItemDetection)
  (params (OverlappedComponent :type Primitive%20Component%20Object%20Reference) (OtherActor :type Actor%20Object%20Reference) (OtherComp :type Primitive%20Component%20Object%20Reference) (OtherBodyIndex :type Integer))
  (Utilities|Array|RemoveItem (Variables|Default|GetInTrayActors) OtherActor)
  (CallFunction|ManageActivationonItemLeave))

(event Custom|RemoveValidateButton
  (Variables|Default|SetDisableButtonIfMoreThanOne true))

(event Custom|Deactivate%20ButtonIfNothingIsIn
  (Variables|Default|SetDisableButtonIfNothingIsIn true)
  (Default|DeactivateButton (Variables|Default|GetValidateButtonRef)))

(event Custom|OnValidateButtonPressed
  (if (Utilities|Array|IsEmpty (Variables|Default|GetInTrayActors))
    (Default|PushTag (Variables|Default|GetTaskManager) "(TagName=\"Task.Flower.EmptyTray\")")
    (elif (Utilities|Array|ContainsItem (Variables|Default|GetInTrayActors) (Game|GetPlayerCharacter 0))
      (Default|PushTag (Variables|Default|GetTaskManager) "(TagName=\"Task.Flower.SelfInside\")")
      (elif (> (Utilities|Array|Length (Variables|Default|GetInTrayActors)) 1)
        (Default|PushTag (Variables|Default|GetTaskManager) "(TagName=\"Task.Flower.TooMushFlowers\")")
        (else
          (bind _asbp_carriable_flower (Utilities|Casting|CastToBP_CarriableFlower (Utilities|Array|Get(acopy) (Variables|Default|GetInTrayActors))))
          (if (Utilities|Enum|Equal(Enum) (Variables|/Game/GameElements/Interractable/Flower/BP_CarriableFlower.BP_CarriableFlower_C|GetFlowerColor _asbp_carriable_flower) "NewEnumerator0")
            (Default|LevelFailed (Variables|Default|GetTaskManager))
            (else
              (Default|PushTag (Variables|Default|GetTaskManager) "(TagName=\"Task.Flower.WrongColor\")"))))))))

(event EventBeginPlay
  (bind _asbp_button (Utilities|Casting|CastToBP_Button (Variables|/Script/Engine.ChildActorComponent|GetChildActor (Variables|Default|GetChildActor_ValidateButton))))
  (Variables|Default|SetValidateButtonRef _asbp_button)
  (Variables|/Game/GameElements/Interractable/BP_Button.BP_Button_C|SetNeedToPressBack (Variables|Default|GetValidateButtonRef) false)
  (Variables|/Game/GameElements/Interractable/BP_Button.BP_Button_C|SetDelayBeforeButtonIsBackInPlace (Variables|Default|GetValidateButtonRef) 0.5)
  (EventDispatchers|BindEventtoOnButtonPressed (Variables|Default|GetValidateButtonRef) (EventDispatchers|CreateEvent :!event Custom|OnValidateButtonPressed)))

(event EventBPIonIncorrectTaskResponseCompleted
  (params (Task :type BP%20Task%20Class%20Class%20Reference))
  (bind _arrayelement (Utilities|Array|ReverseforEachLoop (Variables|Default|GetInTrayActors))
    (:LoopBody
      (Utilities|Casting|CastToBP_Player _arrayelement
        (:CastFailed
          (Utilities|IsValid _arrayelement
            (:Is%20Valid
              (Actor|DestroyActor _arrayelement))))))
    (:Completed
      (Utilities|Array|Clear (Variables|Default|GetInTrayActors)))))

(fn ConstructionScript)

(fn ManageActivatedonItemEnter
  (Utilities|FlowControl|Sequence
    (:then_0
      (Variables|Default|GetDisableButtonIfNothingIsIn
        (:then
          (if (not (Utilities|Array|IsEmpty (Variables|Default|GetInTrayActors)))
            (Default|ActivateButon (Variables|Default|GetValidateButtonRef))))
        (:else)))
    (:then_1
      (Variables|Default|GetDisableButtonIfMoreThanOne
        (:then
          (if (> (Utilities|Array|Length (Variables|Default|GetInTrayActors)) 1)
            (Default|DeactivateButton (Variables|Default|GetValidateButtonRef))))
        (:else)))
    (:then_2
      (return))))

(fn ManageActivationonItemLeave
  (Utilities|FlowControl|Sequence
    (:then_0
      (Variables|Default|GetDisableButtonIfMoreThanOne
        (:then
          (if (< (Utilities|Array|Length (Variables|Default|GetInTrayActors)) 2)
            (Default|ActivateButon (Variables|Default|GetValidateButtonRef))))
        (:else)))
    (:then_1
      (Variables|Default|GetDisableButtonIfNothingIsIn
        (:then
          (if (Utilities|Array|IsEmpty (Variables|Default|GetInTrayActors))
            (Default|DeactivateButton (Variables|Default|GetValidateButtonRef))))
        (:else)))
    (:then_2
      (return))))

(fn PlaySoundifOnlyBlueFlower
  (bind _intrayactors (Variables|Default|GetInTrayActors))
  (bind _asbp_carriable_flower (Utilities|Casting|CastToBP_CarriableFlower (Utilities|Array|Get(acopy) _intrayactors)))
  (if (and (Utilities|Enum|Equal(Enum) (Variables|/Game/GameElements/Interractable/Flower/BP_CarriableFlower.BP_CarriableFlower_C|GetFlowerColor _asbp_carriable_flower) "NewEnumerator0") (== (Utilities|Array|Length _intrayactors) 1))
    (Utilities|FlowControl|DoOnce false
      (:Completed
        (Default|CallPlayLine (Variables|Default|GetFeedbackManager) "/Game/Art/SFX/FlowerVoicelines/SFX_OnBlueFlowerInTray.SFX_OnBlueFlowerInTray")))))

(fn PlaySoundifAllFlowersin
  (bind _intrayactors (Variables|Default|GetInTrayActors))
  (for _array_element _intrayactors
    (Utilities|Casting|CastToBP_CarriableFlower _array_element
      (:CastFailed
        (LocalVariables|SetLocal_AllFlowers false))))
  (if (and (LocalVariables|GetLocal_AllFlowers) (== (Utilities|Array|Length _intrayactors) 3))
    (Utilities|FlowControl|DoOnce false
      (:Completed
        (Default|CallPlayLine (Variables|Default|GetFeedbackManager) "/Game/Art/SFX/FlowerVoicelines/SFX_WholeGardenIn.SFX_WholeGardenIn")))))