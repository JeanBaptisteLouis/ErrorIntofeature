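; Interactable physics prop that the player can pick up into their hand and throw.
; Interact toggles held state: pickup first releases any item the player holds, disables physics and collision, then attaches to the hand.
; A sped-up timeline lerps the relative transform from its captured start into the hand.
; Release detaches it, resets scale, restores physics and launches it along the camera's forward vector.
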(event EventBeginPlay
  (|CallParentFunction)
  (Components|Timeline|SetPlayRate (Variables|Default|GetTM_PickUp) 3.0))

(event EventInterract
  (params (Source :type Actor%20Object%20Reference))
  (bind _mesh (Variables|Character|GetMesh))
  (bind _mesh_2 (Variables|Character|GetMesh))
  (bind _asbp_player (Utilities|Casting|CastToBP_Player Source))
  (Variables|Default|GetHeld
    (:then
      (Variables|Default|SetHeld false)
      (Audio|Components|Audio|Stop (Variables|Default|GetTM_PickUp))
      (Transformation|SetActorRelativeScale3D "1.000000,1.000000,1.000000")
      (Transformation|DetachFromActor "KeepWorld" "KeepWorld" "KeepRelative")
      (Physics|SetSimulatePhysics _mesh true)
      (Collision|SetCollisionEnabled _mesh "QueryAndPhysics")
      (Physics|AddImpulse (Variables|Character|GetMesh) (* (Math|Vector|GetForwardVector (Variables|/Game/Player/BP_Player.BP_Player_C|GetCamera _asbp_player)) 2e+02) "None" true)
      (if (== (Variables|/Game/Player/BP_Player.BP_Player_C|GetHeldActor _asbp_player) self)
        (Variables|/Game/Player/BP_Player.BP_Player_C|SetHeldActor _asbp_player 0)))
    (:else
      (bind _heldactor (Variables|/Game/Player/BP_Player.BP_Player_C|GetHeldActor _asbp_player)
        (:then
          (Class|BPIInterractable|Interract(Message) _heldactor _asbp_player))
        (:else
          _))
      (Variables|Default|SetHeld true)
      (Variables|/Game/Player/BP_Player.BP_Player_C|SetHeldActor _asbp_player self)
      (Physics|SetSimulatePhysics _mesh_2 false)
      (Collision|SetCollisionEnabled _mesh_2 "NoCollision")
      (bind _returnvalue (Transformation|AttachComponentToComponent (Variables|/Game/Player/BP_Player.BP_Player_C|GetHand _asbp_player) "None" "KeepWorld" "KeepWorld" "KeepWorld" true))
      (if _returnvalue
        (Variables|Default|SetPreAnimTransform (Transformation|GetRelativeTransform (Variables|Character|GetMesh)))
        (bind (_direction _alpha) (Timeline|TM_PickUp PlayFromStart)
          (:Update
            (switch Utilities|FlowControl|Switch|SwitchonETimelineDirection _direction
              (:Forward
                (Transformation|SetActorRelativeTransform (Math|Transform|Lerp(Transform) (Variables|Default|GetPreAnimTransform) (Math|Transform|MakeTransform "0, 0, 0" "0, 0, 0" "1.000000,1.000000,1.000000") _alpha) false false)))))))))

(fn ConstructionScript
  (|CallParentFunction))