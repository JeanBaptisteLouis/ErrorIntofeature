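; BP_Button is an interactable button that animates being pushed and fires OnSwitch when activated.
; Interacting toggles Active, playing or reversing the TM_Push timeline that Z-scales AnimScene, with OnSwitch called only on activation.
; Unless OfTypeWitch is set, a finished forward push automatically deactivates and reverses, making the button momentary rather than latching.
; Tick smoothly interpolates the Active state into a material scalar on ButtonMesh.
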(event Custom|Switch
  (Default|CallOnSwitch))

(event EventBeginPlay
  (|CallParentFunction) ; This node is disabled and will not be called.\nDrag off pins to build functionality.
)

(event Collision|EventActorBeginOverlap
  (params (OtherActor :type Actor%20Object%20Reference))
  (|CallParentFunction OtherActor) ; This node is disabled and will not be called.\nDrag off pins to build functionality.
)

(event EventTick
  (params (DeltaSeconds :type Float%20%28single-precision%29))
  (|CallParentFunction DeltaSeconds)
  (bind _output_get (Variables|Default|SetActiveParam (Math|Interpolation|FInterpTo (Variables|Default|GetActiveParam) (Math|Conversions|ToFloat(Boolean) (Variables|Default|GetActive)) DeltaSeconds 1e+01)))
  (Rendering|Material|SetScalarParameterValueonMaterials (Variables|Default|GetButtonMesh) "Active" _output_get))

(event EventInterract
  (params (Source :type Actor%20Object%20Reference))
  (|CallParentFunction Source)
  (Variables|Default|GetActive
    (:then
      (Variables|Default|SetActive false :!label _label)
      (bind (_direction _alpha) (Timeline|TM_Push Reverse)
        (:Update
          (Transformation|SetRelativeScale3D (Variables|Default|GetAnimScene) (Math|Vector|MakeVector 1.0 1.0 _alpha)))
        (:Finished
          (switch Utilities|FlowControl|Switch|SwitchonETimelineDirection _direction
            (:Forward
              (if (not (Variables|Default|GetOfTypeWitch))
                (goto _label)))))))
    (:else
      (Variables|Default|SetActive true)
      (CallFunction|Switch)
      (Timeline|TM_Push Play))))

(fn ConstructionScript
  (|CallParentFunction))