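; BP_Flower is an interactable flower whose mesh takes a blue, yellow or green material from its FlowerColor value.
; The construction script calls SetFlowerColor, which stores the passed color and switches on it to set the mesh's first material slot.
; SetFlowerColorCS repeats the same switch on the stored FlowerColor without taking an input, and is not called within this file.
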(fn ConstructionScript
  (CallFunction|SetFlowerColor (Variables|Color|GetFlowerColor)))

(fn SetFlowerColor
  (params (FlowerColor :type E_FlowerColors%20Enum :default "NewEnumerator0"))
  (bind _output_get (Variables|Color|SetFlowerColor FlowerColor))
  (switch Utilities|FlowControl|Switch|SwitchonE_FlowerColors _output_get
    (:NewEnumerator0
      (Rendering|Material|SetMaterial (Variables|Character|GetMesh) 0 "/Game/Art/M_Color_Blue.M_Color_Blue"))
    (:NewEnumerator1
      (Rendering|Material|SetMaterial (Variables|Character|GetMesh) 0 "/Game/Art/M_Color_Yellow.M_Color_Yellow"))
    (:NewEnumerator2
      (Rendering|Material|SetMaterial (Variables|Character|GetMesh) 0 "/Game/Art/M_Color_Green.M_Color_Green"))))

(fn SetFlowerColorCS
  (switch Utilities|FlowControl|Switch|SwitchonE_FlowerColors (Variables|Color|GetFlowerColor)
    (:NewEnumerator0
      (Rendering|Material|SetMaterial (Variables|Character|GetMesh) 0 "/Game/Art/M_Color_Blue.M_Color_Blue"))
    (:NewEnumerator1
      (Rendering|Material|SetMaterial (Variables|Character|GetMesh) 0 "/Game/Art/M_Color_Yellow.M_Color_Yellow"))
    (:NewEnumerator2
      (Rendering|Material|SetMaterial (Variables|Character|GetMesh) 0 "/Game/Art/M_Color_Green.M_Color_Green"))))