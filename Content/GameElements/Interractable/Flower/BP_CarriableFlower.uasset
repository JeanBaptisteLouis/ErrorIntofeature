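; BP_CarriableFlower is a carriable flower actor that comes in blue, yellow or green.
; The construction script calls SetFlowerColor, which stores the color and swaps the mesh's second material slot to match.
; Hard impacts on the mesh, judged by normal impulse magnitude, play a dropped-flower sound at the actor's location.
; An interface event signalling that an incorrect task response has completed destroys the flower.
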(event OnComponentHit(Mesh)
  (params (HitComponent :type Primitive%20Component%20Object%20Reference) (OtherActor :type Actor%20Object%20Reference) (OtherComp :type Primitive%20Component%20Object%20Reference) (NormalImpulse :type Vector :default "0, 0, 0") (Hit :type Hit%20Result%20Structure%20%28by%20ref%29))
  (if (> (Math|Vector|VectorLength NormalImpulse) 1e+03)
    (Audio|PlaySoundatLocation "/Game/Art/SFX/SFX_FlowerDropped.SFX_FlowerDropped" (Transformation|GetActorLocation) "0, 0, 0" 1.0 1.0 0.0 0 0 0 0)))

(event EventBPIonIncorrectTaskResponseCompleted
  (Actor|DestroyActor))

(fn ConstructionScript
  (CallFunction|SetFlowerColor (Variables|Color|GetFlowerColor)))

(fn SetFlowerColor
  (params (FlowerColor :type E_FlowerColors%20Enum :default "NewEnumerator0"))
  (bind _output_get (Variables|Color|SetFlowerColor FlowerColor))
  (switch Utilities|FlowControl|Switch|SwitchonE_FlowerColors _output_get
    (:NewEnumerator0
      (Rendering|Material|SetMaterial (Variables|Character|GetMesh) 1 "/Game/Art/M_Color_Blue.M_Color_Blue"))
    (:NewEnumerator1
      (Rendering|Material|SetMaterial (Variables|Character|GetMesh) 1 "/Game/Art/M_Color_Yellow.M_Color_Yellow"))
    (:NewEnumerator2
      (Rendering|Material|SetMaterial (Variables|Character|GetMesh) 1 "/Game/Art/M_Color_Green.M_Color_Green"))))