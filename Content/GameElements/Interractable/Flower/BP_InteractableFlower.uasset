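; Pickable flower in the world that hands the interacting source a carriable flower of the same color.
; Interacting spawns a BP_CarriableFlower, passes on color and interaction, then disables and hides this flower with a cut sound.
; When an incorrect task response completes, a picked flower becomes interactable and visible again, with a timeline scale-up pop.
; Construction applies the color enum as a mesh material.
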(event Custom|PopFlower
  (bind _scalelerp (Timeline|FlowerPop PlayFromStart)
    (:Update
      (Transformation|SetWorldScale3D (Variables|Default|GetSM_Flower) (Math|Vector|Lerp(Vector) "0, 0, 0" "1.000000,1.000000,1.000000" _scalelerp)))))

(event EventInterract
  (params (Source :type Actor%20Object%20Reference))
  (bind _returnvalue (Game|SpawnActorfromClass "/Game/GameElements/Interractable/Flower/BP_CarriableFlower.BP_CarriableFlower_C" (Math|Transform|MakeTransform (Transformation|GetWorldLocation (Variables|Default|GetScene)) "0, 0, 0" "1.000000,1.000000,1.000000") "AlwaysSpawn" "MultiplyWithRoot" 0 0))
  (Default|SetFlowerColor _returnvalue (Variables|Color|GetFlowerColor))
  (Default|Interract _returnvalue Source)
  (Variables|Default|SetInterractable false)
  (Development|SetHiddeninGame (Variables|Default|GetSM_Flower) true false)
  (Audio|PlaySoundatLocation "/Game/Art/SFX/SFX_FlowerCut.SFX_FlowerCut" (Transformation|GetActorLocation) "0, 0, 0" 1.0 1.0 0.0 "/Game/Art/SFX/SA_500_1500.SA_500_1500" 0 0 0))

(event EventBPIonIncorrectTaskResponseCompleted
  (Variables|Default|GetInterractable
    (:then)
    (:else
      (Variables|Default|SetInterractable true)
      (Development|SetHiddeninGame (Variables|Default|GetSM_Flower) false false)
      (CallFunction|PopFlower))))

(fn ConstructionScript
  (CallFunction|SetFlowerColor (Variables|Color|GetFlowerColor)))

(fn SetFlowerColor
  (params (FlowerColor :type E_FlowerColors%20Enum :default "NewEnumerator0"))
  (bind _sm_flower (Variables|Default|GetSM_Flower))
  (bind _output_get (Variables|Color|SetFlowerColor FlowerColor))
  (switch Utilities|FlowControl|Switch|SwitchonE_FlowerColors _output_get
    (:NewEnumerator0
      (Rendering|Material|SetMaterial _sm_flower 1 "/Game/Art/M_Color_Blue.M_Color_Blue"))
    (:NewEnumerator1
      (Rendering|Material|SetMaterial _sm_flower 1 "/Game/Art/M_Color_Yellow.M_Color_Yellow"))
    (:NewEnumerator2
      (Rendering|Material|SetMaterial _sm_flower 1 "/Game/Art/M_Color_Green.M_Color_Green"))))

(fn SetFlowerColorCS
  (switch Utilities|FlowControl|Switch|SwitchonE_FlowerColors (Variables|Color|GetFlowerColor)
    (:NewEnumerator0
      (Rendering|Material|SetMaterial (Variables|Character|GetMesh) 0 "/Game/Art/M_Color_Blue.M_Color_Blue"))
    (:NewEnumerator1
      (Rendering|Material|SetMaterial (Variables|Character|GetMesh) 0 "/Game/Art/M_Color_Yellow.M_Color_Yellow"))
    (:NewEnumerator2
      (Rendering|Material|SetMaterial (Variables|Character|GetMesh) 0 "/Game/Art/M_Color_Green.M_Color_Green"))))