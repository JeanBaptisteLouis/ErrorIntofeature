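; BP_Gun is a usable gun that fires BP_Bullet projectiles from its muzzle while ammo remains.
; Use decrements ammo, spawns the bullet with an attached Niagara beam effect, and plays a timeline that drives the actor's relative pitch as a firing kick.
; A DoOnce blocks further shots until that timeline finishes.
; Tick copies the remaining ammo into the W_GunAmmo widget every frame.
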(event EventBeginPlay
  (|CallParentFunction) ; This node is disabled and will not be called.\nDrag off pins to build functionality.
)

(event Collision|EventActorBeginOverlap
  (params (OtherActor :type Actor%20Object%20Reference))
  (|CallParentFunction OtherActor) ; This node is disabled and will not be called.\nDrag off pins to build functionality.
)

(event EventTick
  (params (DeltaSeconds :type Float%20%28single-precision%29))
  (|CallParentFunction DeltaSeconds)
  (bind _asw_gun_ammo (Utilities|Casting|CastToW_GunAmmo (UserInterface|GetWidget (Variables|Default|GetWidget))))
  (Variables|/Game/GameElements/Interractable/Gun/W_GunAmmo.W_GunAmmo_C|SetAmmo _asw_gun_ammo (Variables|Default|GetRemainingAmmo)))

(event EventUse
  (bind _remainingammo (Variables|Default|GetRemainingAmmo))
  (Utilities|FlowControl|DoOnce false :!label _label
    (:Completed
      (if (> _remainingammo 0)
        (Math|Integer|DecrementInt _remainingammo
          (:%20%20
            (Niagara|SpawnSystemAttached "/Game/GameElements/Interractable/Gun/N_Beam.N_Beam" (Variables|Default|GetMuzzle) "None" "0, 0, 0" "0, 0, 0" "KeepRelativeOffset" false)
            (Game|SpawnActorfromClass "/Game/GameElements/Interractable/Gun/BP_Bullet.BP_Bullet_C" (Transformation|GetWorldTransform (Variables|Default|GetMuzzle)) "Undefined" "MultiplyWithRoot" 0 0)
            (bind _alpha (Timeline|TM_Fire PlayFromStart)
              (:Update
                (Transformation|SetActorRelativeRotation (Math|Rotator|MakeRotator 0.0 (* _alpha 1e+01) 0.0)))
              (:Finished
                (goto _label Reset)))))))))

(fn ConstructionScript
  (|CallParentFunction))