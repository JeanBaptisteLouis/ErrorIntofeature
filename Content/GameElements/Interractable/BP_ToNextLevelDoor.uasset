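; Interactable locked door that leads to the next level, opened through the task manager's next-level-unlocked event.
; Interacting shakes the door and counts knocks, triggering scolding voice lines early on and, at ten, pushing a knock task tag and disabling further interaction.
; Opening uses a timeline to lift, rotate and shrink the lock and shrink the door before destroying both.
; The player overlapping the portal plane loads the next level.
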(event OnComponentBeginOverlap(PortalPlane)
  (params (OverlappedComponent :type Primitive%20Component%20Object%20Reference) (OtherActor :type Actor%20Object%20Reference) (OtherComp :type Primitive%20Component%20Object%20Reference) (OtherBodyIndex :type Integer) (bFromSweep :type Boolean) (SweepResult :type Hit%20Result%20Structure%20%28by%20ref%29))
  (Utilities|Casting|CastToBP_Player OtherActor)
  (CallFunction|LoadNextLevel))

(event Custom|VibrateDoor
  (Variables|Default|SetCanInteract false)
  (CallFunction|ManageKnockTask)
  (Audio|PlaySoundatLocation "/Game/Art/SFX/SFX_LockedDoor.SFX_LockedDoor" (Transformation|GetActorLocation) "0, 0, 0" 1.0 1.0 0.0 0 0 0 0)
  (Variables|Default|SetDoorBaseLocation (Transformation|GetWorldLocation (Variables|Default|GetDoorMesh)))
  (bind _movelerp (Timeline|VibrateDoorTimeline PlayFromStart)
    (:Update
      (Transformation|SetWorldLocation (Variables|Default|GetDoorMesh) (Math|Vector|Lerp(Vector) (Variables|Default|GetDoorBaseLocation) (+ (Variables|Default|GetDoorBaseLocation) "0.000000,50.000000,0.000000") _movelerp) false false))
    (:Finished
      (Variables|Default|SetCanInteract (< (Variables|Default|GetKnockDoorCount) 10)))))

(event Custom|OpenDoor
  (Variables|Default|SetCanInteract false)
  (Audio|PlaySoundatLocation "/Game/Art/SFX/SFX_DoorUnlocked.SFX_DoorUnlocked" (Transformation|GetActorLocation) "0, 0, 0" 0.75 1.0 0.0 0 0 0 0)
  (Variables|Default|SetLockBaseLocation (Transformation|GetWorldLocation (Variables|Default|GetLock)))
  (Variables|Default|SetLockBaseRotation (Transformation|GetWorldRotation (Variables|Default|GetLock)))
  (Variables|Default|SetDoorBaseScale (Transformation|GetWorldScale (Variables|Default|GetDoorMesh)))
  (bind (_direction _lockrotatelerp _doorscalelerp _lockmovelerp _lockscalelerp) (Timeline|OpenDoorTimeline PlayFromStart)
    (:Update
      (Transformation|SetWorldRotation (Variables|Default|GetLock) (Math|Rotator|Lerp(Rotator) (Variables|Default|GetLockBaseRotation) (Math|Rotator|MakeRotator (.Roll (Math|Rotator|BreakRotator (Variables|Default|GetLockBaseRotation))) (+ (.Pitch (Math|Rotator|BreakRotator (Variables|Default|GetLockBaseRotation))) 1e+01) (.Yaw (Math|Rotator|BreakRotator (Variables|Default|GetLockBaseRotation)))) _lockrotatelerp true) false false)
      (Transformation|SetWorldScale3D (Variables|Default|GetLock) (Math|Vector|Lerp(Vector) "1.000000,1.000000,1.000000" "0, 0, 0" _lockscalelerp))
      (Transformation|SetWorldLocation (Variables|Default|GetLock) (Math|Vector|Lerp(Vector) (Variables|Default|GetLockBaseLocation) (+ (Variables|Default|GetLockBaseLocation) "0.000000,0.000000,90.000000") _lockmovelerp) false false)
      (Transformation|SetWorldScale3D (Variables|Default|GetDoorMesh) (Math|Vector|Lerp(Vector) (Variables|Default|GetDoorBaseScale) "0, 0, 0" _doorscalelerp)))
    (:Finished
      (Components|DestroyComponent (Variables|Default|GetDoorMesh))
      (Components|DestroyComponent (Variables|Default|GetLock)))))

(event Custom|LoadNextLevel
  (Game|OpenLevel(byObjectReference) (Variables|Default|GetNextLevel)))

(event EventBeginPlay
  (|CallParentFunction)
  (EventDispatchers|BindEventtoOnNextLevelUnlocked (Variables|Default|GetTaskManager_REF) (EventDispatchers|CreateEvent :!event Custom|OpenDoor)))

(event EventBPIonIncorrectTaskResponseCompleted
  (params (Task :type BP%20Task%20Class%20Class%20Reference)))

(event EventInterract
  (params (Source :type Actor%20Object%20Reference))
  (if (Variables|Default|GetCanInteract)
    (|CallParentFunction Source)
    (CallFunction|VibrateDoor)))

(fn ConstructionScript)

(fn ManageKnockTask
  (bind _result (Math|Integer|IncrementInt (Variables|Default|GetKnockDoorCount))
    (:%20%20
      (if (== _result 1)
        (Default|CallPlayLine (Variables|Default|GetFeedbackManager) "/Game/Art/SFX/FlowerVoicelines/SFX_KnockDoor1.SFX_KnockDoor1" "No no, you need to finish this test before entering the next one")
        (elif (== (Variables|Default|GetKnockDoorCount) 3)
          (Default|CallPlayLine (Variables|Default|GetFeedbackManager) "/Game/Art/SFX/FlowerVoicelines/SFX_DoorKnock3rd.SFX_DoorKnock3rd" "What is wrong with you ? Just put my flower in the tray and you'll get through")
          (elif (>= (Variables|Default|GetKnockDoorCount) 10)
            (Default|PushTag (Variables|Default|GetTaskManager_REF) "(TagName=\"Task.Flower.KnockOnDoor\")")))))))