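; BP_TaskManager_1_Flower is a task manager child defining consequences for five incorrect responses to a flower task.
; Each response event applies its effect, then calls the parent handler.
; Effects recolor every flower, remove the item tray's validate button, or deactivate that button when the tray is empty.
; Scissor and jump removal only print placeholders; the recolor response calls its parent once per flower, inside the loop.
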(event EventIncorrectTaskResponse4
  ;[0.15 0.15 0.15 0.5] Put yourself in the item tray
  (Development|PrintString "Remove player jump")
  (|CallParentFunction))

(event EventIncorrectTaskResponse5
  ;[0.15 0.15 0.15 0.5] Rien mettre
  (bind _returnvalue (Actor|GetActorOfClass "/Game/GameElements/BP_ItemTray.BP_ItemTray_C"))
  (Default|DeactivateButtonifNothingIsin _returnvalue)
  (|CallParentFunction))

(event EventIncorrectTaskResponse1
  ;[0.15 0.15 0.15 0.5] Bring back a flower of another color
  (bind _outactors (Actor|GetAllActorsOfClass "/Game/GameElements/Interractable/Flower/BP_Flower.BP_Flower_C"))
  (for _array_element _outactors
    (Default|SetFlowerColor _array_element "NewEnumerator0")
    (|CallParentFunction)))

(event EventIncorrectTaskResponse2
  ;[0.15 0.15 0.15 0.5] Bring back more flowers
  (bind _returnvalue (Actor|GetActorOfClass "/Game/GameElements/BP_ItemTray.BP_ItemTray_C"))
  (Default|RemoveValidateButton _returnvalue)
  (|CallParentFunction))

(event EventIncorrectTaskResponse3
  ;[0.15 0.15 0.15 0.5] Bring back the scissors
  (Development|PrintString "Remove the scissor from the level")
  (|CallParentFunction))

(fn ConstructionScript
  (|CallParentFunction))