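; Task manager that runs a staged target-picking task, spawning one good BP_Target among a crowd of default-setting targets.
; BeginPlay spawns the first wave; separate events trigger three later waves, each clearing existing targets and pausing briefly before respawning.
; Later waves add random movement and change target modes, ending with a big good target in a larger crowd.
; ClearTargets removes all targets, and WrongHit relays to the OnWrongHit dispatcher.
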(event Custom|LastSpawn
  (bind _outactors (Actor|GetAllActorsOfClass "/Game/GameElements/Targets/BP_Target.BP_Target_C"))
  (for _array_element _outactors
    (Default|TargetDone _array_element false))
  (Utilities|FlowControl|Delay 1.0)
  (Game|SpawnActorfromClass "/Game/GameElements/Targets/BP_Target.BP_Target_C" (Math|Transform|MakeTransform "0, 0, 0" "0, 0, 0" "1.000000,1.000000,1.000000") "AlwaysSpawn" "MultiplyWithRoot" 0 false "NewEnumerator0" false true 0)
  (for _index (range 0 28)
    (Game|SpawnActorfromClass "/Game/GameElements/Targets/BP_Target.BP_Target_C" (Math|Transform|MakeTransform "0, 0, 0" "0, 0, 0" "1.000000,1.000000,1.000000") "AlwaysSpawn" "MultiplyWithRoot" 0 true "NewEnumerator1" true false 0)))

(event Custom|WrongHit
  (Default|CallOnWrongHit))

(event Custom|FirstSpawn
  (Game|SpawnActorfromClass "/Game/GameElements/Targets/BP_Target.BP_Target_C" (Math|Transform|MakeTransform "0, 0, 0" "0, 0, 0" "1.000000,1.000000,1.000000") "AlwaysSpawn" "MultiplyWithRoot" 0 false "NewEnumerator3" false false 0)
  (for _index (range 0 24)
    (Game|SpawnActorfromClass "/Game/GameElements/Targets/BP_Target.BP_Target_C" (Math|Transform|MakeTransform "0, 0, 0" "0, 0, 0" "1.000000,1.000000,1.000000") "AlwaysSpawn" "MultiplyWithRoot" 0 true "NewEnumerator3" false false 0)))

(event Custom|SecondSpawn
  (bind _outactors (Actor|GetAllActorsOfClass "/Game/GameElements/Targets/BP_Target.BP_Target_C"))
  (for _array_element _outactors
    (Default|TargetDone _array_element false))
  (Utilities|FlowControl|Delay 1.0)
  (Game|SpawnActorfromClass "/Game/GameElements/Targets/BP_Target.BP_Target_C" (Math|Transform|MakeTransform "0, 0, 0" "0, 0, 0" "1.000000,1.000000,1.000000") "AlwaysSpawn" "MultiplyWithRoot" 0 false "NewEnumerator3" false false 0)
  (for _index (range 0 24)
    (Game|SpawnActorfromClass "/Game/GameElements/Targets/BP_Target.BP_Target_C" (Math|Transform|MakeTransform "0, 0, 0" "0, 0, 0" "1.000000,1.000000,1.000000") "AlwaysSpawn" "MultiplyWithRoot" 0 true "NewEnumerator3" true false 0)))

(event Custom|ThirdSpawn
  (bind _outactors (Actor|GetAllActorsOfClass "/Game/GameElements/Targets/BP_Target.BP_Target_C"))
  (for _array_element _outactors
    (Default|TargetDone _array_element false))
  (Utilities|FlowControl|Delay 1.0)
  (Game|SpawnActorfromClass "/Game/GameElements/Targets/BP_Target.BP_Target_C" (Math|Transform|MakeTransform "0, 0, 0" "0, 0, 0" "1.000000,1.000000,1.000000") "AlwaysSpawn" "MultiplyWithRoot" 0 false "NewEnumerator0" false false 0)
  (for _index (range 0 24)
    (Game|SpawnActorfromClass "/Game/GameElements/Targets/BP_Target.BP_Target_C" (Math|Transform|MakeTransform "0, 0, 0" "0, 0, 0" "1.000000,1.000000,1.000000") "AlwaysSpawn" "MultiplyWithRoot" 0 true "NewEnumerator1" true false 0)))

(event Custom|ClearTargets
  (bind _outactors (Actor|GetAllActorsOfClass "/Game/GameElements/Targets/BP_Target.BP_Target_C"))
  (for _array_element _outactors
    (Default|TargetDone _array_element false)))

(event EventBeginPlay
  (|CallParentFunction)
  (CallFunction|FirstSpawn))

(fn ConstructionScript
  (|CallParentFunction))