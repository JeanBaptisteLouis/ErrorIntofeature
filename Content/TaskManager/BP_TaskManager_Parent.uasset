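; BP_TaskManager_Parent is a base task manager that tracks a level's tasks and signals unlock, completion and failure.
; It spawns each task class on BeginPlay with itself as manager and forwards pushed tags to the running tasks.
; Completions count toward a goal that unlocks the next level once, while finished tasks are pruned until none remain, completing the level.
; Failure broadcasts, then reloads the current level after a short delay.
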(event Custom|LevelComplete
  (Default|CallOnLevelCompleted))

(event Custom|UnlockNextLevel
  (Default|CallOnNextLevelUnlocked))

(event Custom|PushTag
  (params (Tags :type Gameplay%20Tag%20Structure))
  (for _array_element (Variables|Runtime|GetRunningTasks)
    (Default|PushTag _array_element Tags)))

(event Custom|LevelFailed
  (Default|CallOnLevelFailed)
  (Utilities|FlowControl|Delay 3.0)
  (bind _returnvalue (Game|GetCurrentLevelName true))
  (Game|OpenLevel(byName) (Utilities|String|StringToName _returnvalue)))

(event Custom|TaskComplete
  (bind _runningtasks (Variables|Runtime|GetRunningTasks))
  (Utilities|FlowControl|Sequence
    (:then_0
      (bind _result (Math|Integer|IncrementInt (Variables|Runtime|GetCompletedTaskCount))
        (:%20%20
          (if (>= _result (Variables|Default|GetTaskGoal))
            (Utilities|FlowControl|DoOnce false
              (:Completed
                (CallFunction|UnlockNextlevel)))))))
    (:then_1
      (for _array_element _runningtasks
        (if (Variables|/Game/TaskManager/BP_TaskClass.BP_TaskClass_C|GetComplete _array_element)
          (Utilities|Array|RemoveItem _runningtasks _array_element)))
      (Utilities|FlowControl|DelayUntilNextTick)
      (if (Utilities|Array|IsEmpty _runningtasks)
        (CallFunction|LevelComplete)))))

(event EventBeginPlay
  ;[0.15 0.15 0.15 0.5] Init tasks
  (for _array_element (Variables|Default|GetTasks)
    (bind _returnvalue (Game|SpawnActorfromClass _array_element (Math|Transform|MakeTransform "0, 0, 0" "0, 0, 0" "1.000000,1.000000,1.000000") "Undefined" "MultiplyWithRoot" 0 self 0))
    (Utilities|Array|AddUnique (Variables|Runtime|GetRunningTasks) _returnvalue)))

(fn ConstructionScript)