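; BP_TaskClass is a task actor for the task manager, tracking progress through gameplay tags until the task is complete.
; PushTag adds each incoming tag to CompletedTags and calls CompleteTask once that container holds every tag in CompletionTags.
; CompleteTask sets Complete, notifies its Manager, sends a completion message to every BPI_TaskManager actor, then destroys itself after a short delay.
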(event Custom|CompleteTask
  (Variables|Runtime|SetComplete true)
  (Default|TaskComplete (Variables|Default|GetManager))
  (bind _outactors (Actor|GetAllActorswithInterface "/Game/TaskManager/BPI_TaskManager.BPI_TaskManager_C"))
  (for _array_element _outactors
    (Utilities|IsValid _array_element
      (:Is%20Valid
        (Class|BPITaskManager|BPIonIncorrectTaskResponseCompleted(Message) _array_element))))
  (Utilities|FlowControl|Delay 1.0)
  (Actor|DestroyActor))

(event Custom|PushTag
  (params (Tag :type Gameplay%20Tag%20Structure))
  (GameplayTags|AddGameplayTag (Variables|Runtime|GetCompletedTags) Tag :!class /Script/GameplayTags.BlueprintGameplayTagLibrary)
  (if (GameplayTags|HasAllTags (Variables|Runtime|GetCompletedTags) (Variables|Default|GetCompletionTags))
    (CallFunction|CompleteTask)))

(event EventBeginPlay)

(fn ConstructionScript)