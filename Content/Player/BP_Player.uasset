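; First-person player Blueprint that handles Enhanced Input look, move and gated jump, and creates the W_HUD widget.
; Each tick, a thin sphere trace from the camera toggles the HUD interaction prompt according to the hit actor's CanInterractMessage.
; Interact reuses that trace result to send InterractMessage to the target, while Cancel sends the same message to HeldActor, which is set outside this graph.
; A delayed BP_FeedbackManager error-feedback chain is left unconnected.
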(event Input|EnhancedActionEvents|EnhancedInputActionIA_Look
  (params (ActionValue :type Vector%202D%20Structure) (ElapsedSeconds :type Float%20%28double-precision%29) (TriggeredSeconds :type Float%20%28double-precision%29) (InputAction :type Input%20Action%20Object%20Reference :default "/Game/Input/Actions/IA_Look.IA_Look"))
  (Pawn|Input|AddControllerYawInput (.x ActionValue))
  (Pawn|Input|AddControllerPitchInput (* (.y ActionValue) -1.0)))

(event Input|EnhancedActionEvents|EnhancedInputActionIA_Move
  (params (ActionValue :type Vector%202D%20Structure) (ElapsedSeconds :type Float%20%28double-precision%29) (TriggeredSeconds :type Float%20%28double-precision%29) (InputAction :type Input%20Action%20Object%20Reference :default "/Game/Input/Actions/IA_Move.IA_Move"))
  (Pawn|Input|AddMovementInput (Math|Vector|RotateVector (Math|Vector|MakeVector (.y ActionValue) (.x ActionValue) 0.0) (Transformation|GetActorRotation)) 1.0 false))

(event Input|EnhancedActionEvents|EnhancedInputActionIA_Jump
  (params (ActionValue :type Boolean) (ElapsedSeconds :type Float%20%28double-precision%29) (TriggeredSeconds :type Float%20%28double-precision%29) (InputAction :type Input%20Action%20Object%20Reference :default "/Game/Input/Actions/IA_Jump.IA_Jump"))
  (if (and ActionValue (Variables|Default|GetCanPlayerJump))
    (Character|Jump)
    (else
      (Character|StopJumping))))

(event Input|EnhancedActionEvents|EnhancedInputActionIA_Interract
  (params (ActionValue :type Boolean) (ElapsedSeconds :type Float%20%28double-precision%29) (TriggeredSeconds :type Float%20%28double-precision%29) (InputAction :type Input%20Action%20Object%20Reference :default "/Game/Input/Actions/IA_Interract.IA_Interract"))
  (:Started
    (bind _value (Class|BPIInterractable|CanInterract(Message) (.HitActor (Collision|BreakHitResult (stale EventTick _outhit)))))
    (if _value
      (Class|BPIInterractable|Interract(Message) (.HitActor (Collision|BreakHitResult (stale EventTick _outhit))) self))))

(event Input|EnhancedActionEvents|EnhancedInputActionIA_Cancel
  (params (ActionValue :type Boolean) (ElapsedSeconds :type Float%20%28double-precision%29) (TriggeredSeconds :type Float%20%28double-precision%29) (InputAction :type Input%20Action%20Object%20Reference :default "/Game/Input/Actions/IA_Cancel.IA_Cancel"))
  (:Started
    (Class|BPIInterractable|Interract(Message) (Variables|Default|GetHeldActor) self)))

(event EventBeginPlay
  (Input|AddMappingContext (PlayerController|LocalPlayerSubsystems|GetEnhancedInputLocalPlayerSubsystem (Game|GetPlayerController 0)) "/Game/Input/IMC_Default.IMC_Default" 0 "(bIgnoreAllPressedKeysUntilRelease=True,bForceImmediately=False,bNotifyUserSettings=False)")
  (bind _returnvalue (UserInterface|CreateWidget "/Game/Player/UI/W_HUD.W_HUD_C" (Game|GetPlayerController 0)))
  (bind _output_get (Variables|Default|SetHUD _returnvalue))
  (UserInterface|Viewport|AddtoViewport _output_get 0))

(event EventTick
  (params (DeltaSeconds :type Float%20%28single-precision%29))
  (bind _camera (Variables|Default|GetCamera))
  (bind _returnvalue (Transformation|GetWorldLocation _camera))
  (bind (_outhit _returnvalue_2) (Collision|SphereTraceByChannel _returnvalue (+ _returnvalue (* (Math|Vector|GetForwardVector _camera) 2e+02)) 1.0 "TraceTypeQuery1" false 0 "None"))
  (if _returnvalue_2
    (bind _value (Class|BPIInterractable|CanInterract(Message) (.HitActor (Collision|BreakHitResult _outhit))))
    (if _value
      (Default|CanInterract (Variables|Default|GetHUD) true)
      (else
        (Default|CanInterract (Variables|Default|GetHUD) false)))
    (else
      (Default|CanInterract (Variables|Default|GetHUD) false))))

(fn ConstructionScript)