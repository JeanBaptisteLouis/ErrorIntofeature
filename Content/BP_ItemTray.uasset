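; BP_ItemTray is a task tray that judges whether the item placed in it is the correct flower color.
; An overlap box tracks tray contents when a validate button exists, otherwise an overlap triggers validation after a short delay without recording the actor.
; Validation reports coded errors to TaskManager for the player standing inside, a disallowed class, multiple items or wrong color, and success for a matching BP_Flower.
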(event OnComponentBeginOverlap(ItemDetection)
  (params (OverlappedComponent :type Primitive%20Component%20Object%20Reference) (OtherActor :type Actor%20Object%20Reference) (OtherComp :type Primitive%20Component%20Object%20Reference) (OtherBodyIndex :type Integer) (bFromSweep :type Boolean) (SweepResult :type Hit%20Result%20Structure%20%28by%20ref%29))
  (if (Variables|Default|GetHaveValidateButton)
    (Utilities|Array|Add (Variables|Default|GetInTrayActors) OtherActor)
    (else
      (Utilities|FlowControl|Delay 0.2)
      (CallFunction|OnValidateButtonPressed))))

(event OnComponentEndOverlap(ItemDetection)
  (params (OverlappedComponent :type Primitive%20Component%20Object%20Reference) (OtherActor :type Actor%20Object%20Reference) (OtherComp :type Primitive%20Component%20Object%20Reference) (OtherBodyIndex :type Integer))
  (Utilities|Array|RemoveItem (Variables|Default|GetInTrayActors) OtherActor))

(event Custom|RemoveValidateButton)

(event Custom|OnValidateButtonPressed
  (if (Utilities|Array|ContainsItem (Variables|Default|GetInTrayActors) (Game|GetPlayerCharacter 0))
    (Default|OnIncorrectTaskAchieved (Variables|Default|GetTaskManager) 4)
    (else
      (for _array_element (Variables|Default|GetInTrayActors)
        (if (== (Utilities|GetClass _array_element) 0)
          (Default|OnIncorrectTaskAchieved (Variables|Default|GetTaskManager) 3)))
      (if (> (Utilities|Array|Length (Variables|Default|GetInTrayActors)) 1)
        (Default|OnIncorrectTaskAchieved (Variables|Default|GetTaskManager) 2)
        (else
          (bind _asbp_flower (Utilities|Casting|CastToBP_Flower (Utilities|Array|Get(acopy) (Variables|Default|GetInTrayActors))))
          (if (Utilities|Enum|Equal(Enum) (Variables|/Game/BP_Flower.BP_Flower_C|GetFlowerColor _asbp_flower) "NewEnumerator0")
            (Default|OnCorrectTaskAchieved (Variables|Default|GetTaskManager))
            (else
              (Default|OnIncorrectTaskAchieved (Variables|Default|GetTaskManager) 1))))))))

(fn ConstructionScript)