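; BP_FeedbackManager gives the player voice-line and error feedback.
; Shortly after BeginPlay it caches the player's HUD and plays the Click_on_Button line.
; PlayLine plays a 2D sound, shows the sound asset's name as fixed-duration HUD dialog text, then waits out the sound's length.
; ErrorFeedback runs a timeline that drives the Error scalar in the MPC_Feedback material parameter collection.
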(event Custom|ErrorFeedback
  (bind _alpha (Timeline|TM_ErrorFB PlayFromStart)
    (:Update
      (Rendering|Material|SetScalarParameterValue "/Game/Art/Feedback/MPC_Feedback.MPC_Feedback" "Error" _alpha :!class /Script/Engine.KismetMaterialLibrary))))

(event EventBeginPlay
  (Utilities|FlowControl|Delay 0.1)
  (bind _asbp_player (Utilities|Casting|CastToBP_Player (Game|Player|GetPlayerPawn 0)))
  (Variables|Default|SetHUD (Variables|/Game/Player/BP_Player.BP_Player_C|GetHUD _asbp_player))
  (Utilities|FlowControl|Delay 0.2)
  (Utilities|PlayLine "/Engine/VREditor/Sounds/UI/Click_on_Button.Click_on_Button"))

(fn ConstructionScript)